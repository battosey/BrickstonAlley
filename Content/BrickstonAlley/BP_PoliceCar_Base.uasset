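; BP_PoliceCar_Base is a base police car Blueprint that exposes control over its flasher and emergency lights.
; GetLightForAddress maps a light address to one of the car's front, mirror, side, rear, roof flasher or turret lights through a Select node.
; ChangeLight resolves the address through that lookup and forwards emission level, color and on/off state to the chosen light.
; The construction script is empty.
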(fn `ChangeLight`
  (params (LightAddress :type "/Game/BrickstonAlley/Data/ELightAddress Enum" :default "NewEnumerator0") (FlasherEmissionLevel :type "Float (double-precision)") (Color :type "Color Structure") (bIsOn :type Boolean))
  (`/Game/BrickstonAlley/Lights/BP_LightBallComponent.ChangeLight` (`self.GetLightForAddress` LightAddress) FlasherEmissionLevel Color bIsOn))

(fn `GetLightForAddress`
  (params (LightAddress :type "/Game/BrickstonAlley/Data/ELightAddress Enum" :default "NewEnumerator0"))
  (returns (ReturnValue :type "/Game/BrickstonAlley/Lights/BP_LightBallComponent Object Reference"))
  (return (select `/Game/BrickstonAlley/Data/ELightAddress` (`local.LightAddress`) :`NewEnumerator0` (`self.Flasher_FL1`) :`NewEnumerator1` (`self.Flasher_FL2`) :`NewEnumerator2` (`self.Flasher_FL3`) :`NewEnumerator3` (`self.Flasher_LMirr`) :`NewEnumerator4` (`self.Flasher_L1`) :`NewEnumerator5` (`self.Flasher_L2`) :`NewEnumerator6` (`self.Flasher_RL1`) :`NewEnumerator7` (`self.Flasher_RL2`) :`NewEnumerator8` (`self.Flasher_RL3`) :`NewEnumerator9` (`self.Flasher_TopL3`) :`NewEnumerator10` (`self.Flasher_TopL4`) :`NewEnumerator11` (`self.Flasher_TopL1`) :`NewEnumerator12` (`self.Flasher_TopL2`) :`NewEnumerator13` (`self.Flasher_TopL5`) :`NewEnumerator14` (`self.Flasher_TopL8`) :`NewEnumerator15` (`self.Flasher_TopL7`) :`NewEnumerator16` (`self.Flasher_TopL6`) :`NewEnumerator17` (`self.Flasher_FR1`) :`NewEnumerator18` (`self.Flasher_FR2`) :`NewEnumerator19` (`self.Flasher_FR3`) :`NewEnumerator20` (`self.Flasher_RMirr`) :`NewEnumerator21` (`self.Flasher_R1`) :`NewEnumerator22` (`self.Flasher_R2`) :`NewEnumerator23` (`self.Flasher_RR1`) :`NewEnumerator24` (`self.Flasher_RR2`) :`NewEnumerator25` (`self.Flasher_RR3`) :`NewEnumerator26` (`self.Flasher_TopR8`) :`NewEnumerator27` (`self.Flasher_TopR7`) :`NewEnumerator32` (`self.Flasher_TopR5`) :`NewEnumerator33` (`self.Flasher_TopR3`) :`NewEnumerator28` (`self.Flasher_TopR1`) :`NewEnumerator29` (`self.Flasher_TopR4`) :`NewEnumerator30` (`self.Flasher_TopR6`) :`NewEnumerator31` (`self.Flasher_TopR2`) :`NewEnumerator34` (`self.Turret_LF`) :`NewEnumerator35` (`self.Turret_LM`) :`NewEnumerator36` (`self.Turret_LR`) :`NewEnumerator37` (`self.Turret_RF`) :`NewEnumerator38` (`self.Turret_RM`) :`NewEnumerator39` (`self.Turret_RR`))))

(fn `UserConstructionScript`)