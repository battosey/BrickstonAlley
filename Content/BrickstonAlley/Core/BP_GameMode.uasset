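; Game mode for the BrickstonAlley level that keeps the police car nearest the screen center set as the demo car.
; On BeginPlay and every Tick it projects all BP_PoliceCar_Base actors to screen space and passes the one closest to the viewport center to SetDemoCar.
; A separate helper, GetLightAddresses, converts a list of light names into matching ELightAddress values by iterating the enum.
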(event `self.ReceiveBeginPlay`
  (`self.SelectClosestCarToCenterAsDemoCar` :!label _label))

(event `self.ReceiveTick`
  (params (DeltaSeconds :type "Float (single-precision)"))
  (goto _label))

(fn `GetLightAddresses`
  (params (LightNames :type "Array of Name (by ref)"))
  (returns (LightAddresses :type "Array of /Game/BrickstonAlley/Data/ELightAddress Enum"))
  (locals (Result :type "Array of /Game/BrickstonAlley/Data/ELightAddress Enum"))
  (bind _enumvalue (foreach `/Game/BrickstonAlley/Data/ELightAddress` false)
    (:`LoopBody`
      (if (`KismetArrayLibrary.Array_Contains` LightNames (`/Game/BrickstonAlley/Data/BFL_LightUtils.GetLightName` _enumvalue))
        (`KismetArrayLibrary.Array_Add` (`local.Result`) _enumvalue)))
    (:`then`
      (return (`local.Result`)))))

(fn `SelectClosestCarToCenterAsDemoCar`
  (locals (ClosestDist :type "Float (double-precision)" :default 0.0) (ClosestCar :type "/Game/BrickstonAlley/BP_PoliceCar_Base Object Reference"))
  (bind _returnvalue (`GameplayStatics.GetPlayerController` 0))
  (bind (_sizex _sizey) (`PlayerController.GetViewportSize` _returnvalue))
  (bind _outactors (`GameplayStatics.GetAllActorsOfClass` "/Game/BrickstonAlley/BP_PoliceCar_Base.BP_PoliceCar_Base_C"))
  (for _array_element _outactors
    (bind (_screenposition _returnvalue_2) (`GameplayStatics.ProjectWorldToScreen` _returnvalue (`self.K2_GetActorLocation` _array_element)))
    (if _returnvalue_2
      (bind _returnvalue_3 (`KismetMathLibrary.DistanceSquared2D` _screenposition (/ (`KismetMathLibrary.MakeVector2D` (`KismetMathLibrary.Conv_IntToDouble` _sizex) (`KismetMathLibrary.Conv_IntToDouble` _sizey)) (2.0 2.0))))
      (if (or (< _returnvalue_3 (`local.ClosestDist`)) (not (`KismetSystemLibrary.IsValid` (`local.ClosestCar`))))
        (set `local.ClosestDist` _returnvalue_3)
        (set `local.ClosestCar` _array_element))))
  (bind _closestcar (`local.ClosestCar`)
    (:`then`
      (`self.SetDemoCar` _closestcar))
    (:`else`)))

(fn `UserConstructionScript`)